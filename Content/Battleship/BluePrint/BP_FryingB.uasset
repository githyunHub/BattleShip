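; BP_FryingB is a player-flown propeller aircraft that drops BP_Missile actors just below itself on left mouse click.
; Thrust, MoveUp and MoveRight axes drive clamped forward speed and interpolated pitch, yaw and roll speeds, which Tick applies as local movement and rotation while spinning both propellers.
; Yaw feeds banking roll and slight pitch, roll self-levels without steering, and hits nudge the rotation toward the surface normal.
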(event `Key|LeftMouseButton`
  (params (Key :type "Key Structure"))
  (bind (_returnvalue_x _returnvalue_y _returnvalue_z) (`KismetMathLibrary.BreakVector` (`self.K2_GetActorLocation`)))
  (:`Pressed`
    (`|SpawnActorFromClass` "/Game/Battleship/BluePrint/BP_Missile.BP_Missile_C" (`KismetMathLibrary.MakeTransform` (`KismetMathLibrary.MakeVector` _returnvalue_x _returnvalue_y (- _returnvalue_z 50.0))) "Undefined" "OverrideRootScale" null null)))

(event `self.ReceiveTick`
  (params (DeltaSeconds :type "Float (single-precision)"))
  (bind _returnvalue (`GameplayStatics.GetWorldDeltaSeconds`))
  (`self.K2_AddActorLocalOffset` (`KismetMathLibrary.MakeVector` (* DeltaSeconds (`self.Current forward speed`))))
  (`self.K2_AddActorLocalRotation` (`KismetMathLibrary.MakeRotator` (* _returnvalue (`self.Current roll speed`)) (* _returnvalue (`self.Current pitch speed`)) (* _returnvalue (`self.Current yaw speed`))))
  (`SceneComponent.K2_AddRelativeRotation` (`self.SM_P38_Propeller`) (`KismetMathLibrary.MakeRotator` (* _returnvalue (`self.PropellerSpeed`))) false false)
  (`SceneComponent.K2_AddRelativeRotation` (`self.SM_P38_Propeller1`) (`KismetMathLibrary.MakeRotator` (* _returnvalue (`self.PropellerSpeed`))) false false))

(event `InputAxis|Thrust`
  (params (AxisValue :type "Float (single-precision)"))
  (bind _acceleration (`self.Acceleration`))
  (set `self.Current forward speed` (`KismetMathLibrary.FClamp` (+ (`self.Current forward speed`) (* (`KismetMathLibrary.SelectFloat` (* AxisValue _acceleration) (* _acceleration -0.5) (!= AxisValue 0.0)) (`GameplayStatics.GetWorldDeltaSeconds`))) (`self.Min speed`) (`self.MaxSpeed`))) ; Update forward speed based on input axis value
)

(event `InputAxis|MoveUp`
  (params (AxisValue :type "Float (single-precision)"))
  (set `self.Current pitch speed` (`KismetMathLibrary.FInterpTo` (`self.Current pitch speed`) (+ (* AxisValue (`self.Turn speed`) -1.0) (* (`KismetMathLibrary.Abs` (`self.Current yaw speed`)) -0.2)) (`GameplayStatics.GetWorldDeltaSeconds`) 2.0)) ; Update pitch speed based on input axis value and yaw speed
)

(event `InputAxis|MoveRight`
  (params (AxisValue :type "Float (single-precision)"))
  (set `self.Current yaw speed` (`KismetMathLibrary.FInterpTo` (`self.Current yaw speed`) (* AxisValue (`self.Turn speed`)) (`GameplayStatics.GetWorldDeltaSeconds`) 2.0)) ; Update yaw speed based on input axis value
  (set `self.Current roll speed` (`KismetMathLibrary.FInterpTo` (`self.Current roll speed`) (`KismetMathLibrary.SelectFloat` (* (`self.Current yaw speed`) 0.5) (* (.roll (`self.K2_GetActorRotation`)) -2.0) (> (`KismetMathLibrary.Abs` AxisValue) 0.2)) (`GameplayStatics.GetWorldDeltaSeconds`) 2.0)) ; Update rolls speed based on yaw speed
)

(event `self.ReceiveHit`
  (params (MyComp :type "PrimitiveComponent Object Reference") (Other :type "Actor Object Reference") (OtherComp :type "PrimitiveComponent Object Reference") (bSelfMoved :type Boolean) (HitLocation :type "Vector Structure") (HitNormal :type "Vector Structure") (NormalImpulse :type "Vector Structure") (Hit :type "HitResult Structure (by ref)"))
  ;[1 1 1] Deflect when colliding
  (`self.K2_SetActorRotation` (`KismetMathLibrary.RLerp` (`self.K2_GetActorRotation`) (`KismetMathLibrary.Conv_VectorToRotator` HitNormal) 0.025 true)))

(fn `UserConstructionScript`)